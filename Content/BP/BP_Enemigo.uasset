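; Enemy character that chases the player, attacks on arrival and dies after enough hits from BP_Proyectil01.
; After a random start delay, Seguir loops AI MoveTo: success plays AtaqueEnemigo01's montage and effect and makes Tick face the player, failure retries later.
; AtaqueEnemigo02 spawns an enemy projectile but is not called here.
; Hits play feedback and subtract health after a delay; death triggers animation, increments the player's NumEnemigos and destroys the enemy.
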(event OnComponentBeginOverlap(CapsuleComponent)
  (params (OverlappedComponent :type Primitive%20Component%20Object%20Reference) (OtherActor :type Actor%20Object%20Reference) (OtherComp :type Primitive%20Component%20Object%20Reference) (OtherBodyIndex :type Integer) (bFromSweep :type Boolean) (SweepResult :type Hit%20Result%20Structure%20%28by%20ref%29))
  (bind _as_bp_player (Variables|Default|GetAs%20BP%20Player))
  ;[0.15 0.15 0.15 0.5] ColisionProyectil
  (Utilities|IsValid OtherActor
    (:Is%20Valid
      (bind _asbp_proyectil_01 (Utilities|Casting|CastToBP_Proyectil01 OtherActor))
      (Class|NiagaraComponent|SetAsset (Variables|/Game/BP/BP_Proyectil01.BP_Proyectil01_C|GetNiagara _asbp_proyectil_01) "/Game/Basic_VFX/Niagara/NS_Basic_3.NS_Basic_3" true)
      (Audio|PlaySound2D "/Game/FreeModularMagicSFX/F_Examples/MSS_MagicExample_Shooting_Crystal.MSS_MagicExample_Shooting_Crystal" 1.0 1.0 0.0 0 0)
      (Animation|PlayAnimMontage "/Game/Characters/Enemigo/Anim/Mon_hit.Mon_hit" 1.0 "None")
      (Audio|PlaySound2D "/Game/HumanVocalizations/HumanFemaleA/Cues/voice_female_a_battle_shout_09_Cue.voice_female_a_battle_shout_09_Cue" 1.0 1.0 0.0 0 0)
      (Actor|DestroyActor _asbp_proyectil_01)
      (Utilities|FlowControl|Delay 2.0)
      (Variables|Default|Setvida_enemigo (- (Variables|Default|Getvida_enemigo) 1))
      (if (<= (Variables|Default|Getvida_enemigo) 0)
        (bind _asanim_enemigo (Utilities|Casting|CastToAnim_Enemigo (Components|SkeletalMesh|GetAnimInstance (Variables|Character|GetMesh))))
        (Audio|PlaySound2D "/Game/HumanVocalizations/HumanFemaleA/Wavs/voice_female_a_battle_shout_04.voice_female_a_battle_shout_04" 1.0 1.0 0.0 0 0)
        (Variables|/Game/Characters/Enemigo/Anim/Anim_Enemigo.Anim_Enemigo_C|Setmuerte _asanim_enemigo true)
        (Pawn|Components|CharacterMovement|DisableMovement (Variables|Character|GetCharacterMovement))
        (Utilities|FlowControl|Delay 4.0)
        (Variables|/Game/ThirdPerson/Blueprints/BP_Player.BP_Player_C|SetnumEnemigos _as_bp_player (+ (Variables|/Game/ThirdPerson/Blueprints/BP_Player.BP_Player_C|GetnumEnemigos _as_bp_player) 1))
        (Actor|DestroyActor)))))

(event Custom|Seguir
  ;[0.15 0.15 0.15 0.5] Seguir
  (AI|AIMoveTo self "0, 0, 0" (Game|GetPlayerCharacter 0) 6e+01 false
    (:OnSuccess
      (Variables|Default|SetAtacar true)
      (CallFunction|AtaqueEnemigo01)
      (Utilities|FlowControl|Delay 4.0)
      (CallFunction|Seguir))
    (:OnFail
      (Variables|Default|SetAtacar false)
      (Utilities|FlowControl|Delay (Math|Random|RandomFloatinRange 9.0 27.0))
      (CallFunction|Seguir))))

(event Custom|AtaqueEnemigo01
  ;[0.15 0.15 0.15 0.5] AtaqueEnemigo01
  (Class|NiagaraComponent|SetAsset (Variables|Default|GetNiagara) "/Game/Basic_VFX/Niagara/NS_Basic_7.NS_Basic_7" true)
  (Animation|PlayAnimMontage "/Game/Characters/Enemigo/Anim/Mon_atq.Mon_atq" 1.0 "None"))

(event Custom|AtaqueEnemigo02
  ;[0.15 0.15 0.15 0.5] AtaqueEnemigo02
  (Game|SpawnActorfromClass "/Game/BP/BP_ProyectilEnm.BP_ProyectilEnm_C" (Transformation|GetWorldTransform (Variables|Default|GetArrow_projectil)) "Undefined" "MultiplyWithRoot" 0 0))

(event EventBeginPlay
  (bind _returnvalue (Game|GetPlayerCharacter 0))
  (Utilities|IsValid _returnvalue
    (:Is%20Valid
      (bind _asbp_player (Utilities|Casting|CastToBP_Player _returnvalue))
      (Variables|Default|SetAs%20BP%20Player _asbp_player)
      (Utilities|Time|SetTimerbyFunctionName 0 "Seguir" (Math|Random|RandomFloatinRange 4.0 9.0)))))

(event EventTick
  (params (DeltaSeconds :type Float%20%28single-precision%29))
  (if (Variables|Default|GetAtacar)
    (Transformation|SetWorldRotation (Variables|Collision|GetCapsuleComponent) (Math|Rotator|FindLookatRotation (Transformation|GetWorldLocation (Variables|Collision|GetCapsuleComponent)) (Transformation|GetActorLocation (Variables|Default|GetAs%20BP%20Player))) false false)))

(fn ConstructionScript)